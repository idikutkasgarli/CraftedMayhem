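; Item pile for a pick-up game that belongs to one character and collects BaseItem actors.
; While the pile is unfilled, its owning avatar entering the player trigger makes that player's controller drop its item.
; Items entering the item trigger are tagged with this pile and passed to AddToPile, whose result sets Filled.
; When that result is true, the game mode runs PileCheck.
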(event OnComponentBeginOverlap(TriggerBoxForPlayer)
  (params (OverlappedComponent :type Primitive%20Component%20Object%20Reference) (OtherActor :type Actor%20Object%20Reference) (OtherComp :type Primitive%20Component%20Object%20Reference) (OtherBodyIndex :type Integer) (bFromSweep :type Boolean) (SweepResult :type Hit%20Result%20Structure%20%28by%20ref%29))
  (if (not (Variables|Default|GetFilled))
    (bind _asbp_net_avatar (Utilities|Casting|CastToBP_NetAvatar OtherActor))
    (if (== _asbp_net_avatar (Variables|Default|GetBelongCharacter))
      (bind _aspc_net_player (Utilities|Casting|CastToPC_NetPlayer (Pawn|GetController _asbp_net_avatar)))
      (Default|DropItemInput _aspc_net_player))))

(event OnComponentBeginOverlap(TriggerBox)
  (params (OverlappedComponent :type Primitive%20Component%20Object%20Reference) (OtherActor :type Actor%20Object%20Reference) (OtherComp :type Primitive%20Component%20Object%20Reference) (OtherBodyIndex :type Integer) (bFromSweep :type Boolean) (SweepResult :type Hit%20Result%20Structure%20%28by%20ref%29))
  (bind _asbase_item (Utilities|Casting|CastToBaseItem OtherActor))
  (CallFunction|SetBaseItemProperties _asbase_item)
  (bind _bfilled (Class|ItemPile|AddtoPile _asbase_item))
  (bind _output_get (Variables|Default|SetFilled _bfilled))
  (if _output_get
    (Default|PileCheck (Variables|Default|GetAs%20BP%20Pick%20Up%20Game))))

(event EventBeginPlay
  (bind _asgm_pick_up_game (Utilities|Casting|CastToGM_PickUpGame (Game|GetGameMode)))
  (Variables|Default|SetAs%20BP%20Pick%20Up%20Game _asgm_pick_up_game))

(event Collision|EventActorBeginOverlap
  (params (OtherActor :type Actor%20Object%20Reference))
  (Utilities|FlowControl|Sequence))

(event EventTick
  (params (DeltaSeconds :type Float%20%28single-precision%29))
  (Networking|SwitchHasAuthority))

(fn ConstructionScript)

(fn SetBaseItemProperties
  (params (Last%20Item%20Pile%20In :type Base%20Item%20Object%20Reference))
  (Variables|/Script/LabWork4.BaseItem|SetLastItemPileIn Last%20Item%20Pile%20In self)
  (Variables|/Script/LabWork4.BaseItem|SetbWasInPile Last%20Item%20Pile%20In true))