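; Lobby game mode that launches the PickItemGame match once the required player count is reached.
; On PostLogin it compares LastPlayerID to TotalPlayerToStart, then reads the body-part selection from player 0's BP_NetAvatar.
; With authority, it passes that selection and an empty nickname to NetGameInstance's Host call.
; Disconnected leftover nodes hold a per-player loop, a debug print and a localhost Join.
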(event EventPostLogin
  (params (NewPlayer :type Player%20Controller%20Object%20Reference))
  (|CallParentFunction NewPlayer)
  (if (== (Variables|Default|GetLastPlayerID) (Variables|Default|GetTotalPlayerToStart))
    (bind _asbp_net_avatar (Utilities|Casting|CastToBP_NetAvatar (Game|Player|GetPlayerPawn 0)))
    (Networking|SwitchHasAuthority
      (:Authority
        (Class|NetGameInstance|Host (.AsNet%20Game%20Instance (Utilities|Casting|CastToNetGameInstance (Game|GetGameInstance))) "PickItemGame" (Utilities|Struct|MakeSPlayerInfo "" (Variables|/Script/LabWork4.NetBaseCharacter|GetPartSelection _asbp_net_avatar)))))))

(fn ConstructionScript
  (|CallParentFunction))