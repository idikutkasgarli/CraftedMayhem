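; Networked player avatar that swings a sword on left mouse and shows a world-space health bar.
; Attacks route to the server, where timelines rotate the sword and its pivot, alternating swing direction.
; While swinging, Tick sphere-traces between blade sockets and applies damage.
; Incoming damage passes a DoOnce gate, reset on the server after a short delay, and multicasts the health bar, which starts hidden and faces the camera.
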(event Custom|HealthBarServer
  (CallFunction|HealthBarMultiCast))

(event Custom|HealthBarMultiCast
  (Progress|SetPercent (Variables|Default|GetHealth%20Bar) (/ (Variables|Default|GetHealth) (Variables|Default|GetMaxHealth))))

(event Custom|SetHealthBarVisibility
  (params (Visible :type Boolean))
  (CallFunction|ServerSetHealthbarVis Visible))

(event Custom|ServerSetHealthbarVis
  (params (Visibility :type Boolean))
  (CallFunction|MultiCastSetHealthBarVis Visibility))

(event Custom|MultiCastSetHealthBarVis
  (params (Visibility :type Boolean))
  (bind _health_bar (Variables|Default|GetHealth%20Bar)
    (:then
      (if Visibility
        (Widget|SetVisibility _health_bar "Visible")
        (else
          (Widget|SetVisibility _health_bar "Hidden"))))
    (:else)))

(event Custom|SwordUp
  (bind _sworddownalpha (Timeline|Timeline PlayFromStart)
    (:Update
      (Transformation|SetRelativeRotation (Variables|Default|GetSword) (Math|Rotator|MakeRotator (Math|Float|Lerp (Variables|Default|GetSword%20Rotation%20X%20%28Roll%29) 0.0 _sworddownalpha) (Variables|Default|GetSword%20Rotation%20Y%20%28Pitch%29) (Variables|Default|GetSword%20Rotation%20Z%20%28Yaw%29)) false false))))

(event Custom|RunOnServer_SwordAttack
  (bind _hitspeed (Variables|Default|GetHitSpeed))
  (if (not (Variables|Default|GetPlayingAnimSword))
    (Utilities|FlowControl|Sequence
      (:then_0
        (|SwordUpRotation _hitspeed))
      (:then_1
        (|SwordPivotRotation _hitspeed)))))

(event Custom|RunOnServerDead)

(event EventBeginPlay
  (bind _aswbp_health_bar (Utilities|Casting|CastToWBP_HealthBar (UserInterface|GetWidget (Variables|Default|GetHealthBarWidget))))
  (Variables|Default|SetHealth%20Bar (Variables|/Game/Blueprints/Widgets/WBP_HealthBar.WBP_HealthBar_C|GetHealthBar _aswbp_health_bar))
  (CallFunction|SetHealthBarVisibility false)
  (bind _aspc_net_player (Utilities|Casting|CastToPC_NetPlayer (Pawn|GetController)))
  (Variables|Default|SetPlayerController _aspc_net_player))

(event EventUnpossessed
  (params (OldController :type Controller%20Object%20Reference)))

(event EventTick
  (params (DeltaSeconds :type Float%20%28single-precision%29))
  (bind _sword (Variables|Default|GetSword))
  (bind _healthbarwidget (Variables|Default|GetHealthBarWidget))
  (Transformation|SetWorldRotation _healthbarwidget (Math|Rotator|FindLookatRotation (Transformation|GetWorldLocation _healthbarwidget) (Transformation|GetWorldLocation (Variables|/Script/Engine.Actor|GetRootComponent (Game|GetPlayerCameraManager 0)))) false false)
  (if (Variables|Default|GetPlayingAnimSword)
    (bind _outhit (Collision|SphereTraceByChannel (Transformation|GetSocketLocation _sword "swordStart") (Transformation|GetSocketLocation _sword "swordEnd") 15.0 "TraceTypeQuery1" false 0 "ForOneFrame"))
    (Game|Damage|ApplyDamage (.HitActor (Collision|BreakHitResult _outhit)) 2e+01 0 0)))

(event Game|Damage|EventAnyDamage
  (params (Damage :type Float%20%28single-precision%29) (DamageType :type Damage%20Type%20Object%20Reference) (InstigatedBy :type Controller%20Object%20Reference) (DamageCauser :type Actor%20Object%20Reference))
  (Utilities|FlowControl|DoOnce false :!label _label
    (:Completed
      (Class|NetBaseCharacter|TakeDamage Damage DamageType InstigatedBy DamageCauser)
      (Networking|SwitchHasAuthority
        (:Authority
          (CallFunction|HealthBarServer)
          (Utilities|FlowControl|Delay 0.4)
          (goto _label Reset))))))

(event Input|MouseEvents|DebugKeyLeftMouseButton
  (params (Key :type Key%20Structure :default "None") (ActionValue :type Input%20Action%20Value%20Structure))
  (bind _hitspeed (Variables|Default|GetHitSpeed))
  (:Pressed
    (Networking|SwitchHasAuthority
      (:Authority
        (if (not (Variables|Default|GetPlayingAnimSword))
          (Utilities|FlowControl|Sequence
            (:then_0
              (|SwordUpRotation _hitspeed))
            (:then_1
              (|SwordPivotRotation _hitspeed)))))
      (:Remote
        (CallFunction|RunonServerSwordAttack)))))

(fn ConstructionScript)

(fn GetSelfController
  (bind _aspc_net_player (Utilities|Casting|CastToPC_NetPlayer (Game|GetPlayerController (Variables|/Game/Blueprints/BP_PlayerState.BP_PlayerState_C|GetPlayerIndex (.AsBP%20Player%20State (Utilities|Casting|CastToBP_PlayerState (Variables|Default|GetPlayerState)))))))
  (return _aspc_net_player))

(fn OnRepBHoldingAnItem)

(fn OnRepHealthBar)