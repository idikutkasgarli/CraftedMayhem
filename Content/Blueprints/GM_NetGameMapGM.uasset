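; Game mode for a networked map that gives each new player an avatar and moves on to the PickItemGame session.
; HandleStartingNewPlayer spawns and possesses a BP_NetAvatar, then checks whether LastPlayerID equals TotalPlayerToStart.
; On a match, it passes player 0's body-part selection and a placeholder nickname to NetGameInstance.
; An authority switch chooses between hosting and joining a hardcoded LAN address.
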(event EventHandleStartingNewPlayer
  (params (NewPlayer :type Player%20Controller%20Object%20Reference))
  (bind _returnvalue (Game|GetGameInstance))
  (bind _asnet_game_instance (Utilities|Casting|CastToNetGameInstance _returnvalue))
  (|CallParentFunction NewPlayer)
  (bind _returnvalue_2 (Game|SpawnActorfromClass "/Game/Blueprints/BP_NetAvatar.BP_NetAvatar_C" (Math|Transform|MakeTransform "0, 0, 0" "0, 0, 0" "1.000000,1.000000,1.000000") "Undefined" "MultiplyWithRoot" 0 0))
  (Pawn|Possess NewPlayer _returnvalue_2)
  (if (== (Variables|Default|GetLastPlayerID) (Variables|Default|GetTotalPlayerToStart))
    (bind _asbp_net_avatar (Utilities|Casting|CastToBP_NetAvatar (Game|Player|GetPlayerPawn 0)))
    (Development|PrintString "sasasa" true true "(R=1.000000,G=0.000000,B=0.149247,A=1.000000)" 2222.0)
    (Networking|SwitchHasAuthority
      (:Authority
        (Class|NetGameInstance|Host _asnet_game_instance "PickItemGame" (Utilities|Struct|MakeSPlayerInfo "a" (Variables|/Script/LabWork4.NetBaseCharacter|GetPartSelection _asbp_net_avatar))))
      (:Remote
        (Class|NetGameInstance|Join _asnet_game_instance "192.168.1.102" (Utilities|Struct|MakeSPlayerInfo "a" (Variables|/Script/LabWork4.NetBaseCharacter|GetPartSelection _asbp_net_avatar)))))))

(event EventPostLogin
  (params (NewPlayer :type Player%20Controller%20Object%20Reference))
  (|CallParentFunction NewPlayer))

(fn ConstructionScript
  (|CallParentFunction))