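; BP_PickUpGame is a game mode for a pick-up game that places up to four players at numbered player starts.
; On each new player, it restarts everyone in Players by index, gathers their BP_NetAvatar pawns into AllPawns, then calls SetCharacterPiles.
; When the pawn count reaches TotalPlayerToStart, it hides all their health bars after a short delay.
; Tick prints every gathered pawn's name on screen as debug output.
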(event EventHandleStartingNewPlayer
  (params (NewPlayer :type Player%20Controller%20Object%20Reference))
  (|CallParentFunction NewPlayer)
  (for (_array_element _array_index) (Variables|Default|GetPlayers)
    (if (== _array_index 0)
      (Class|GameModeBase|RestartPlayeratPlayerStart _array_element (Class|GameModeBase|FindPlayerStart _array_element "0"))
      (bind _asbp_net_avatar (Utilities|Casting|CastToBP_NetAvatar (Pawn|GetControlledPawn _array_element) :!label _label))
      (bind _returnvalue (Utilities|Array|AddUnique (Variables|Default|GetAllPawns) _asbp_net_avatar))
      (if (== (+ _returnvalue 1) (Variables|Default|GetTotalPlayerToStart))
        (Utilities|FlowControl|Delay 0.2)
        (for _array_element_2 (Variables|Default|GetAllPawns)
          (Default|SetHealthBarVisibility _array_element_2 false)))
      (elif (== _array_index 1)
        (Class|GameModeBase|RestartPlayeratPlayerStart _array_element (Class|GameModeBase|FindPlayerStart _array_element "1"))
        (goto _label)
        (elif (== _array_index 2)
          (Class|GameModeBase|RestartPlayeratPlayerStart _array_element (Class|GameModeBase|FindPlayerStart 0 "2"))
          (goto _label)
          (elif (== _array_index 3)
            (Class|GameModeBase|RestartPlayeratPlayerStart _array_element (Class|GameModeBase|FindPlayerStart 0 "3"))
            (goto _label))))))
  (Default|CallSetCharacterPiles))

(event EventTick
  (params (DeltaSeconds :type Float%20%28single-precision%29))
  (|CallParentFunction DeltaSeconds)
  (for _array_element (Variables|Default|GetAllPawns)
    (Development|PrintString (Utilities|GetDisplayName _array_element) true true "(R=0.000000,G=1.000000,B=0.607947,A=1.000000)" DeltaSeconds)))

(event EventPostLogin
  (params (NewPlayer :type Player%20Controller%20Object%20Reference))
  (|CallParentFunction NewPlayer))

(event EventBeginPlay
  (|CallParentFunction) ; This node is disabled and will not be called.\nDrag off pins to build functionality.
)

(fn ConstructionScript
  (|CallParentFunction))