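; BP_GetPlayerPiles is a helper Blueprint meant to assign in-game piles to players, though its assignment logic is currently disconnected and BeginPlay is empty.
; The unused authority-only chain matches each pile by index to BP_PickUpGame's PlayerPawns, up to LastPlayerID, and sets BelongCharacter with debug prints.
; It then calls SetLocationServer, which forwards to SetLocationMulti to move that pawn to a fixed point above the world origin.
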(event Custom|SetLocationServer
  (params (Character :type BP%20Net%20Avatar%20Object%20Reference))
  (CallFunction|SetLocationMulti Character))

(event Custom|SetLocationMulti
  (params (Character :type BP%20Net%20Avatar%20Object%20Reference))
  (Transformation|SetActorTransform Character (Math|Transform|MakeTransform "0.000000,0.000000,1000.000000" "0, 0, 0" "1.000000,1.000000,1.000000")))

(event EventBeginPlay)

(fn ConstructionScript)