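; Network player controller that lets a player drop a held item with the 1 key.
; The key branches on authority: the authority side clears HasItem and calls the DropItem dispatcher directly.
; The remote side goes through the ClientDrop event, which calls DropItem only if HasItem is set and leaves the flag unchanged.
; The bDropItemClient RepNotify is empty, and the DropItemClient call, player-index check and debug print are unconnected leftovers.
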(event Custom|ClientDrop
  (if (Variables|Default|GetbHasItem)
    (Default|CallDropItem)))

(event EventBeginPlay)

(event EventTick
  (params (DeltaSeconds :type Float%20%28single-precision%29)))

(event Input|KeyboardEvents|1
  (params (Key :type Key%20Structure :default "None"))
  (:Pressed
    (Networking|SwitchHasAuthority
      (:Authority
        (Variables|Default|SetbHasItem false)
        (Default|CallDropItem))
      (:Remote
        (CallFunction|ClientDrop)))))

(fn ConstructionScript)

(fn OnRepBDropItemClient)