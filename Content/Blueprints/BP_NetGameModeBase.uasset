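; BP_NetGameModeBase is a multiplayer game mode that registers joining players and places them at numbered player starts.
; HandleStartingNewPlayer adds each controller to Players and gives its BP_PlayerState an incrementing PlayerIndex.
; SetPlayerStarts restarts the first four players at tagged starts matching their array position, via PlayerStartCheck, and collects their BP_NetAvatar pawns into AllPawns.
; Nothing in this file calls SetPlayerStarts.
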(event EventBeginPlay)

(event EventTick
  (params (DeltaSeconds :type Float%20%28single-precision%29)))

(event EventPostLogin
  (params (NewPlayer :type Player%20Controller%20Object%20Reference)))

(event EventHandleStartingNewPlayer
  (params (NewPlayer :type Player%20Controller%20Object%20Reference))
  (bind _lastplayerid (Variables|Default|GetLastPlayerID))
  (Utilities|Array|Add (Variables|Default|GetPlayers) NewPlayer)
  (bind _asbp_player_state (Utilities|Casting|CastToBP_PlayerState (Variables|/Script/Engine.Controller|GetPlayerState NewPlayer)))
  (Variables|/Game/Blueprints/BP_PlayerState.BP_PlayerState_C|SetPlayerIndex _asbp_player_state _lastplayerid)
  (Math|Integer|IncrementInt _lastplayerid))

(fn ConstructionScript)

(fn SetPlayerStarts
  (for (_array_element _array_index) (Variables|Default|GetPlayers)
    (CallFunction|PlayerStartCheck _array_element _array_index)
    (bind _asbp_net_avatar (Utilities|Casting|CastToBP_NetAvatar (Pawn|GetControlledPawn _array_element)))
    (Utilities|Array|AddUnique (Variables|Default|GetAllPawns) _asbp_net_avatar))
  (return))

(fn PlayerStartCheck
  (params (Player :type Controller%20Object%20Reference) (A :type Integer))
  (if (== A 0)
    (Class|GameModeBase|RestartPlayeratPlayerStart Player (Class|GameModeBase|FindPlayerStart Player "0"))
    (elif (== A 1)
      (Class|GameModeBase|RestartPlayeratPlayerStart Player (Class|GameModeBase|FindPlayerStart Player "1"))
      (elif (== A 2)
        (Class|GameModeBase|RestartPlayeratPlayerStart Player (Class|GameModeBase|FindPlayerStart 0 "2"))
        (elif (== A 3)
          (Class|GameModeBase|RestartPlayeratPlayerStart Player (Class|GameModeBase|FindPlayerStart 0 "3")))))))