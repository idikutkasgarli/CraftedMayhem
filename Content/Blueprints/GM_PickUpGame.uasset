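; Game mode for the networked pick-up stage, where filled piles lead into combat.
; As players join, it sets starts and character piles, then hides health bars once all expected pawns exist.
; When PileCheck counts two filled piles, it respawns and repossesses an avatar per player, then hosts CombatLvl using player 0's body parts and stats.
; Tick prints every pawn's name as debug output.
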(event Custom|PileCheck
  (bind _result (Math|Integer|IncrementInt (Variables|Default|GetFilledPiles))
    (:%20%20
      (if (== _result 2)
        (bind _asbp_net_avatar (Utilities|Casting|CastToBP_NetAvatar (Game|Player|GetPlayerPawn 0)))
        (Variables|Default|SetPart%20Selection (Variables|/Script/LabWork4.NetBaseCharacter|GetPartSelection _asbp_net_avatar))
        (Variables|Default|SetPlayer%20Stats (Variables|/Script/LabWork4.NetBaseCharacter|GetPlayerStats _asbp_net_avatar))
        (Utilities|Array|Clear (Variables|Default|GetAllPawns))
        (for (_array_element _array_index) (Variables|Default|GetNew%20Player)
          (Pawn|UnPossess _array_element)
          (bind _returnvalue (Game|SpawnActorfromClass "/Game/Blueprints/BP_NetAvatar.BP_NetAvatar_C" (Math|Transform|MakeTransform "0, 0, 0" "0, 0, 0" "1.000000,1.000000,1.000000") "Undefined" "MultiplyWithRoot" 0 0))
          (Utilities|Array|Add (Variables|Default|GetAllPawns) _returnvalue)
          (Pawn|Possess _array_element _returnvalue)
          (bind _aspc_net_player (Utilities|Casting|CastToPC_NetPlayer _array_element))
          (Variables|/Script/LabWork4.NetBaseCharacter|SetPlayerController (Utilities|Array|Get(acopy) (Variables|Default|GetAllPawns) _array_index) _aspc_net_player))
        (Networking|SwitchHasAuthority
          (:Authority
            (Class|NetGameInstance|Host (.AsNet%20Game%20Instance (Utilities|Casting|CastToNetGameInstance (Game|GetGameInstance))) "CombatLvl" (Utilities|Struct|MakeSPlayerInfo "a" (Variables|Default|GetPart%20Selection)) (Variables|Default|GetPlayer%20Stats))))))))

(event Custom|SetHealthBar
  (for _array_element (Variables|Default|GetAllPawns)
    (Default|SetHealthBarVisibility _array_element false)
    (Development|PrintString "yav")))

(event EventHandleStartingNewPlayer
  (params (NewPlayer :type Player%20Controller%20Object%20Reference))
  (Utilities|Array|Add (Variables|Default|GetNew%20Player) NewPlayer)
  (|CallParentFunction NewPlayer)
  (CallFunction|SetPlayerStarts)
  (Default|CallSetCharacterPiles)
  (if (== (Utilities|Array|Length (Variables|Default|GetAllPawns)) (Variables|Default|GetTotalPlayerToStart))
    (Utilities|FlowControl|Delay 0.3)
    (for _array_element (Variables|Default|GetAllPawns)
      (Default|SetHealthBarVisibility _array_element false))))

(event EventTick
  (params (DeltaSeconds :type Float%20%28single-precision%29))
  (|CallParentFunction DeltaSeconds)
  (for _array_element (Variables|Default|GetAllPawns)
    (Development|PrintString (Utilities|GetDisplayName _array_element) true true "(R=0.000000,G=1.000000,B=0.607947,A=1.000000)" DeltaSeconds)))

(event EventPostLogin
  (params (NewPlayer :type Player%20Controller%20Object%20Reference))
  (|CallParentFunction NewPlayer))

(event EventBeginPlay
  (|CallParentFunction) ; This node is disabled and will not be called.\nDrag off pins to build functionality.
)

(fn ConstructionScript
  (|CallParentFunction))